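; Player tank Blueprint that handles camera aiming input and firing.
; On BeginPlay it passes its barrel and turret components to SetBarrelReference and SetTurretReference, which are defined outside this graph.
; Horizontal aim input yaws a gimbal and vertical input pitches the spring arm, keeping the two rotation axes on separate components.
; The Fire action calls Fire, also defined outside the file.
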(event `self.ReceiveBeginPlay`
  (`self.SetBarrelReference` (`self.Tank_Barrel`))
  (`self.SetTurretReference` (`self.Tank_Turret`)))

(event `InputAxis|AimHorizontal`
  (params (AxisValue :type "Float (single-precision)"))
  ;[1 1 1] Horizontal Movement
  (`SceneComponent.K2_AddLocalRotation` (`self.Horizontal Gimbal`) (`KismetMathLibrary.MakeRotator` 0.0 0.0 (* AxisValue 1.0)) false false))

(event `InputAction|Fire`
  (params (Key :type "Key Structure"))
  (:`Pressed`
    (`self.Fire`)))

(event `InputAxis|AimVertical`
  (params (AxisValue :type "Float (single-precision)"))
  ;[1 1 1] Vertical Movement
  (`SceneComponent.K2_AddLocalRotation` (`self.SpringArm`) (`KismetMathLibrary.MakeRotator` 0.0 (* AxisValue 1.0)) false false))

(fn `UserConstructionScript`)